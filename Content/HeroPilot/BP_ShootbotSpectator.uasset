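; BP_ShootbotSpectator is a spectator pawn that moves the view in the world Y-Z plane.
; MoveRight and MoveUp axis inputs feed scaled world-space vectors into a FloatingPawnMovement component, with the horizontal axis inverted.
; On BeginPlay, the ArmExtend timeline pulls the camera back by lerping the SpringArm length from its start value to a fixed distance beyond it.
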(event Custom|ExtendCameraArm
  (Variables|Default|SetArmLengthFinish (+ (Variables|Default|GetArmLengthStart) 3e+02))
  (bind _blendval (Timeline|ArmExtend PlayFromStart)
    (:Update
      (Variables|/Script/Engine.SpringArmComponent|SetTargetArmLength (Variables|Default|GetSpringArm) (Math|Float|Lerp (Variables|Default|GetArmLengthStart) (Variables|Default|GetArmLengthFinish) _blendval)))))

(event EventBeginPlay
  (CallFunction|ExtendCameraArm))

(event Collision|EventActorBeginOverlap
  (params (OtherActor :type Actor%20Object%20Reference)))

(event EventTick
  (params (DeltaSeconds :type Float%20%28single-precision%29)))

(event Input|AxisEvents|InputAxisMoveRight
  (params (AxisValue :type Float%20%28single-precision%29))
  (Class|PawnMovementComponent|AddInputVector (Variables|Default|GetFloatingPawnMovement) (Math|Vector|MakeVector 0.0 (* AxisValue (Variables|Default|GetAxisScalar) -1.0) 0.0) false))

(event Input|AxisEvents|InputAxisMoveUp
  (params (AxisValue :type Float%20%28single-precision%29))
  (Class|PawnMovementComponent|AddInputVector (Variables|Default|GetFloatingPawnMovement) (Math|Vector|MakeVector 0.0 0.0 (* AxisValue (Variables|Default|GetAxisScalar))) false))

(fn ConstructionScript)