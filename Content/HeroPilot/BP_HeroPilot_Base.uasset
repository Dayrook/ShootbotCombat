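; Base Blueprint for the hero pilot, a plane-constrained side-scrolling character who fights on foot or from inside a mech.
; Entering disables collision and floats the capsule to the mech's Cockpit socket by timeline, then hides the pilot and pins it there on Tick.
; While piloting, move, jump and light attack inputs forward to MyMech; on foot they drive walking, jetpack impulses and bullet spawning.
; Exiting ejects the pilot along the mech's facing with a brief jetpack boost.
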(event Custom|Exit%20Mech
  ;[1 1 1] Enter / Exit Mech
  (CallFunction|Eject (Variables|Default|GetMyMech))
  (Default|LosePilot (Variables|Default|GetMyMech))
  (Variables|Default|SetInMech false)
  (Rendering|SetVisibility (Variables|Character|GetMesh) true true)
  (Collision|SetCollisionEnabled (Variables|Default|GetCapsuleComponent) "QueryAndPhysics"))

(event Custom|Enter%20Mech
  ;[1 1 1] Enter / Exit Mech
  (CallFunction|JumpPilotEnd)
  (Collision|SetCollisionEnabled (Variables|Default|GetCapsuleComponent) "NoCollision")
  (Variables|Default|SetStartingLocation (Transformation|GetWorldLocation (Variables|Default|GetCapsuleComponent)))
  (bind _floatval (Timeline|FloatToChest PlayFromStart)
    (:Update
      (Transformation|SetWorldLocation (Variables|Default|GetCapsuleComponent) (Math|Vector|MakeVector (Variables|Default|GetPlane_Constraint) (.y (Math|Vector|Lerp(Vector) (Variables|Default|GetStartingLocation) (Transformation|GetSocketLocation (Variables|/Script/Engine.Character|GetMesh (Variables|Default|GetMyMech)) "Cockpit") _floatval)) (.z (Math|Vector|Lerp(Vector) (Variables|Default|GetStartingLocation) (Transformation|GetSocketLocation (Variables|/Script/Engine.Character|GetMesh (Variables|Default|GetMyMech)) "Cockpit") _floatval))) false false))
    (:Finished
      (Default|GetPilot (Variables|Default|GetMyMech))
      (Variables|Default|SetInMech true)
      (Rendering|SetVisibility (Variables|Character|GetMesh) false true))))

(event Custom|Jump_Pilot_Start
  ;[1 1 1] Movement
  (Variables|Default|SetJetpackActive true)
  (Components|Activation|SetActive (Variables|Default|GetJetpackExhaust) true false))

(event Custom|Eject
  (params (EjectingMech :type BP%20Hero%20Mech%20Base%20Object%20Reference))
  ;[1 1 1] Eject
  (CallFunction|MovetoCockpit)
  (Variables|/Script/Engine.MovementComponent|SetVelocity (Variables|Character|GetCharacterMovement) (Math|Vector|MakeVector 0.0 (select (> (.y (Math|Vector|GetForwardVector (Variables|/Script/Engine.Character|GetCapsuleComponent EjectingMech))) 0.0) 3.5e+02 -3.5e+02) 0.0))
  (Variables|Default|SetJetpackActive true)
  (Utilities|FlowControl|Delay 0.5)
  ;;[1 1 1] Player Doesn't Want To Jetpack
  (if (not (Components|Activation|IsActive (Variables|Default|GetJetpackExhaust)))
    (CallFunction|JumpPilotEnd)))

(event Custom|Jump_Pilot_End
  ;[1 1 1] Movement
  (Variables|Default|SetJetpackActive false)
  (Components|Activation|SetActive (Variables|Default|GetJetpackExhaust) false false))

(event EventTick
  (params (DeltaSeconds :type Float%20%28single-precision%29))
  ;[1 1 1] Tick: Stay In Cockpit, JetPackBoost
  (if (Variables|Default|GetInMech)
    (Utilities|IsValid (Variables|Default|GetMyMech)
      (:Is%20Valid
        (CallFunction|MovetoCockpit)))
    (elif (Variables|Default|GetJetpackActive)
      (Physics|AddImpulse (Variables|Character|GetCharacterMovement) (Math|Vector|MakeVector 0.0 (* (.y (Math|Vector|GetForwardVector (Variables|Default|GetCapsuleComponent))) 2e+01) (Variables|Default|GetJetpackStrength)) false))))

(event Input|ActionEvents|InputActionEnter/ExitMech
  (params (Key :type Key%20Structure))
  ;[1 1 1] Enter / Exit Mech
  (:Pressed
    (if (Variables|Default|GetInMech)
      (CallFunction|ExitMech)
      (else
        (CallFunction|EnterMech)))))

(event Input|ActionEvents|InputActionJump
  (params (Key :type Key%20Structure))
  ;[1 1 1] Movement
  (:Pressed
    (if (Variables|Default|GetInMech)
      (Character|Jump (Variables|Default|GetMyMech))
      (else
        (CallFunction|JumpPilotStart))))
  (:Released
    (if (Variables|Default|GetInMech)
      (Character|StopJumping (Variables|Default|GetMyMech))
      (else
        (CallFunction|JumpPilotEnd)))))

(event Input|ActionEvents|InputActionAttack_Light
  (params (Key :type Key%20Structure))
  ;[1 1 1] Attack
  (:Pressed
    (if (Variables|Default|GetInMech)
      (Default|PAttackLight (Variables|Default|GetMyMech))
      (else
        (bind _returnvalue (Game|SpawnActorfromClass "/Game/Weapons/BP_PilotBullet.BP_PilotBullet_C" (Math|Transform|MakeTransform (Transformation|GetWorldLocation (Variables|Default|GetCapsuleComponent)) "0, 0, 0" "1,1,1") "Undefined" 0 0))
        (Utilities|Array|Add (Variables|/Game/Weapons/BP_BulletBase.BP_BulletBase_C|GetIgnorables _returnvalue) self)
        (Utilities|Array|Add (Variables|/Game/Weapons/BP_BulletBase.BP_BulletBase_C|GetIgnorables _returnvalue) (Variables|Default|GetMyMech))
        (Variables|/Game/Weapons/BP_BulletBase.BP_BulletBase_C|SetSpeed _returnvalue (select (>= (.y (Math|Vector|GetForwardVector (Variables|Default|GetCapsuleComponent))) 0.0) 1.5e+02 -1.5e+02))))))

(event Input|AxisEvents|InputAxisMoveRight
  (params (AxisValue :type Float%20%28single-precision%29))
  (bind _returnvalue (* -1 AxisValue))
  ;[1 1 1] Movement
  (if (Variables|Default|GetInMech)
    (Pawn|Input|AddMovementInput (Variables|Default|GetMyMech) (Math|Vector|MakeVector 0.0 _returnvalue 0.0) 1.0 false)
    (else
      (Pawn|Input|AddMovementInput (Math|Vector|MakeVector 0.0 _returnvalue 0.0) 1.0 false) ; C++ equivalent: AddMovementInput(FVector(0.f,-1.f,0.f), Value);
    )))

(fn ConstructionScript)

(fn MovetoCockpit
  (bind _mymech (Variables|Default|GetMyMech))
  (bind _mesh (Variables|/Script/Engine.Character|GetMesh _mymech))
  (bind _returnvalue (Transformation|GetSocketLocation _mesh "Cockpit"))
  (Transformation|SetWorldLocation (Variables|Default|GetCapsuleComponent) (Math|Vector|MakeVector (Variables|Default|GetPlane_Constraint) (.y _returnvalue) (.z _returnvalue)) false false))