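; BP_MechSpawner keeps a hero mech at its spot, spawning a BP_HeroMech_Base whenever none overlaps its Box.
; A slow Tick drives the overlap check, which retries after a delay while occupied.
; Spawns use the static mesh's Y and Z on the MechPlane X.
; MechTypeNumber selects mesh and animation overrides applied after spawning; the class is fixed, and the mech type is noted as not replicating.
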(event Custom|ConfigureMech
  ;[1 1 1] Set up Mech. Still not replicating mech type
  (Variables|ShootbotVarietal|SetMechTypeNumber (Math|Integer|Clamp(Integer) (Variables|ShootbotVarietal|GetMechTypeNumber) 0 1))
  (Utilities|FlowControl|Delay 0.2)
  (Variables|Default|SetMechType "/Game/HeroMech/BP_HeroMech_Base.BP_HeroMech_Base_C")
  (Variables|Default|SetOverwriteMesh (Utilities|Select :Index (Variables|ShootbotVarietal|GetMechTypeNumber) :Option%200 "/Game/Mannequin/Character/Mesh/SK_Mannequin.SK_Mannequin" :Option%201 "/Engine/Tutorial/SubEditors/TutorialAssets/Character/TutorialTPP.TutorialTPP"))
  (Variables|Default|SetOverwriteAnimation (Utilities|Select :Index (Variables|ShootbotVarietal|GetMechTypeNumber) :Option%200 "/Game/Mannequin/Animations/ABP_Mech.ABP_Mech_C" :Option%201 "/Game/HeroMech/ABP_TutorialTPP.ABP_TutorialTPP_C")))

(event Custom|TrySpawnMech
  (bind _staticmesh (Variables|Default|GetStaticMesh))
  (bind _overwritemesh (Variables|Default|GetOverwriteMesh))
  (bind _returnvalue (Transformation|GetWorldLocation _staticmesh))
  (Variables|/Script/Engine.PrimitiveComponent|SetbGenerateOverlapEvents (Variables|Default|GetBox) true)
  (if (< (Utilities|Array|Length (Collision|GetOverlappingActors (Variables|Default|GetBox) "/Game/HeroMech/BP_HeroMech_Base.BP_HeroMech_Base_C" :!class /Script/Engine.PrimitiveComponent)) 1)
    (bind _returnvalue_2 (Game|SpawnActorfromClass (Variables|Default|GetMechType) (Math|Transform|MakeTransform (Math|Vector|MakeVector (Variables|Default|GetMechPlane) (.y _returnvalue) (+ (.z _returnvalue) 0.0)) "0,90.000000, 0" "1,1,1") "Undefined" 0 0))
    (Variables|/Script/Engine.PrimitiveComponent|SetbGenerateOverlapEvents (Variables|Default|GetBox) false)
    (Utilities|IsValid _overwritemesh
      (:Is%20Valid
        (bind _asbp_hero_mech_base (Utilities|Casting|CastToBP_HeroMech_Base _returnvalue_2))
        (Class|SkinnedMeshComponent|SetSkeletalMesh (Variables|/Script/Engine.Character|GetMesh _asbp_hero_mech_base) _overwritemesh true)
        (if (Utilities|IsValidClass (Variables|Default|GetOverwriteAnimation))
          (Components|SkeletalMesh|SetAnimInstanceClass (Variables|/Script/Engine.Character|GetMesh _asbp_hero_mech_base) (Variables|Default|GetOverwriteAnimation)))))
    (else
      (Utilities|FlowControl|Delay 3.0)
      (CallFunction|TrySpawnMech))))

(event EventBeginPlay
  ;[1 1 1] Set up Mech. Still not replicating mech type
  (CallFunction|ConfigureMech))

(event EventTick
  (params (DeltaSeconds :type Float%20%28single-precision%29))
  ;[1 1 1] SLOW TICK
  (CallFunction|TrySpawnMech))

(fn ConstructionScript)