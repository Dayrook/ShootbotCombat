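; Base hero pawn that moves along the world Y axis on foot and can pilot its own mech.
; Entering disables collision, floats the capsule to the mech's Cockpit socket via a timeline, then hides the hero and registers it as pilot.
; While piloting, Tick pins the capsule to the mech and move, jump and light attack inputs forward to it.
; On foot, light attack fires a facing-based bullet that ignores hero and mech.
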(event Custom|Exit%20Mech
  ;[1 1 1] Enter / Exit Mech
  (Collision|SetCollisionEnabled (Variables|Default|GetCapsuleComponent) "QueryAndPhysics")
  (Default|LosePilot (Variables|Default|GetMyMech))
  (Variables|Default|SetInMech false)
  (Rendering|SetVisibility (Variables|Character|GetMesh) true true))

(event Custom|Enter%20Mech
  ;[1 1 1] Enter / Exit Mech
  (Collision|SetCollisionEnabled (Variables|Default|GetCapsuleComponent) "NoCollision")
  (Variables|Default|SetStartingLocation (Transformation|GetWorldLocation (Variables|Default|GetCapsuleComponent)))
  (bind _floatval (Timeline|FloatToChest PlayFromStart)
    (:Update
      (Transformation|SetWorldLocation (Variables|Default|GetCapsuleComponent) (Math|Vector|Lerp(Vector) (Variables|Default|GetStartingLocation) (Transformation|GetSocketLocation (Variables|/Script/Engine.Character|GetMesh (Variables|Default|GetMyMech)) "Cockpit") _floatval) false false))
    (:Finished
      (Default|GetPilot (Variables|Default|GetMyMech))
      (Variables|Default|SetInMech true)
      (Rendering|SetVisibility (Variables|Character|GetMesh) false true))))

(event EventTick
  (params (DeltaSeconds :type Float%20%28single-precision%29))
  (bind _mymech (Variables|Default|GetMyMech))
  ;[1 1 1] Stay In Cockpit
  (if (Variables|Default|GetInMech)
    (Utilities|IsValid _mymech
      (:Is%20Valid
        (Transformation|SetWorldLocation (Variables|Default|GetCapsuleComponent) (Transformation|GetWorldLocation (Variables|/Script/Engine.Character|GetCapsuleComponent _mymech)) false false)))))

(event Input|ActionEvents|InputActionEnter/ExitMech
  (params (Key :type Key%20Structure))
  ;[1 1 1] Enter / Exit Mech
  (:Pressed
    (if (Variables|Default|GetInMech)
      (CallFunction|ExitMech)
      (else
        (CallFunction|EnterMech)))))

(event Input|ActionEvents|InputActionJump
  (params (Key :type Key%20Structure))
  ;[1 1 1] Movement
  (:Pressed
    (if (Variables|Default|GetInMech)
      (Character|Jump (Variables|Default|GetMyMech))
      (else
        (Character|Jump))))
  (:Released
    (if (Variables|Default|GetInMech)
      (Character|StopJumping (Variables|Default|GetMyMech))
      (else
        (Character|StopJumping)))))

(event Input|ActionEvents|InputActionAttack_Light
  (params (Key :type Key%20Structure))
  (:Pressed
    (if (Variables|Default|GetInMech)
      (Default|PAttackLight (Variables|Default|GetMyMech))
      (else
        (bind _returnvalue (Game|SpawnActorfromClass "/Game/Weapons/BP_PersonBullet.BP_PersonBullet_C" (Math|Transform|MakeTransform (Transformation|GetWorldLocation (Variables|Default|GetCapsuleComponent)) "0, 0, 0" "1,1,1") "Undefined" 0 0))
        (Utilities|Array|Add (Variables|/Game/Weapons/BP_BulletBase.BP_BulletBase_C|GetIgnorables _returnvalue) self)
        (Utilities|Array|Add (Variables|/Game/Weapons/BP_BulletBase.BP_BulletBase_C|GetIgnorables _returnvalue) (Variables|Default|GetMyMech))
        (Variables|/Game/Weapons/BP_BulletBase.BP_BulletBase_C|SetSpeed _returnvalue (select (>= (.y (Math|Vector|GetForwardVector (Variables|Default|GetCapsuleComponent))) 0.0) 1.5e+02 -1.5e+02))))))

(event Input|AxisEvents|InputAxisMoveRight
  (params (AxisValue :type Float%20%28single-precision%29))
  (bind _returnvalue (* -1 AxisValue))
  ;[1 1 1] Movement
  (if (Variables|Default|GetInMech)
    (Pawn|Input|AddMovementInput (Variables|Default|GetMyMech) (Math|Vector|MakeVector 0.0 _returnvalue 0.0) 1.0 false)
    (else
      (Pawn|Input|AddMovementInput (Math|Vector|MakeVector 0.0 _returnvalue 0.0) 1.0 false) ; C++ equivalent: AddMovementInput(FVector(0.f,-1.f,0.f), Value);
    )))

(fn ConstructionScript)