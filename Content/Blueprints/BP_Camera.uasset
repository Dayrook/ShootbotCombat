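; BP_Camera is a follow camera Blueprint that tracks a target along the Y and Z axes while holding a fixed depth on X, as in a side-scroller.
; BeginPlay caches the scene component's starting world X.
; Each Tick moves that component to the cached X and the FollowTarget capsule's Y and Z, with a fixed upward offset and no smoothing.
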(event EventBeginPlay
  (Variables|Default|SetStartX (.x (Transformation|GetWorldLocation (Variables|Default|GetSceneComponent)))))

(event EventTick
  (params (DeltaSeconds :type Float%20%28single-precision%29))
  (bind _followtarget (Variables|Default|GetFollowTarget))
  (bind _capsulecomponent (Variables|/Script/Engine.Character|GetCapsuleComponent _followtarget))
  (bind _returnvalue (Transformation|GetWorldLocation _capsulecomponent))
  (Transformation|SetWorldLocation (Variables|Default|GetSceneComponent) (Math|Vector|MakeVector (Variables|Default|GetStartX) (.y _returnvalue) (+ (.z _returnvalue) 4e+01)) false false))

(fn ConstructionScript)