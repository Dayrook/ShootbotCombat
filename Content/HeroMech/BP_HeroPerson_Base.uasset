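; BP_HeroPerson_Base is the base Blueprint for the on-foot hero who can enter and exit a mech.
; The Enter / Exit Mech input either unpossesses the hero, calls GetPilot on MyMech and disables capsule collision, or repossesses the hero and restores collision and camera.
; While InMech, Tick moves the hero's capsule to the mech's capsule location.
; BeginPlay sets the view target to MyCamera.
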(event Custom|Exit%20Mech
  (Pawn|Possess (Game|GetPlayerController (Variables|Default|GetMyPlayerID)) self)
  (Variables|Default|SetInMech false)
  ;[1 1 1] TODO: Remove
  (CallFunction|GrabCamera)
  (Collision|SetCollisionEnabled (Variables|Default|GetCapsuleComponent) "QueryAndPhysics"))

(event Custom|Enter%20Mech
  (Pawn|UnPossess (Game|GetPlayerController (Variables|Default|GetMyPlayerID)))
  (Default|GetPilot (Variables|Default|GetMyMech))
  (Variables|Default|SetInMech true)
  (Collision|SetCollisionEnabled (Variables|Default|GetCapsuleComponent) "NoCollision"))

(event Custom|GrabCamera
  (Variables|Default|SetbFindCameraComponentWhenViewTarget true)
  (Game|Player|SetViewTargetwithBlend (Game|GetPlayerController 0) (Variables|Default|GetMyCamera) 0.0 "VTBlend_Linear" 0.0 false))

(event EventTick
  (params (DeltaSeconds :type Float%20%28single-precision%29))
  (bind _mymech (Variables|Default|GetMyMech))
  (if (Variables|Default|GetInMech)
    (Utilities|IsValid _mymech
      (:Is%20Valid
        (Transformation|SetWorldLocation (Variables|Default|GetCapsuleComponent) (Transformation|GetWorldLocation (Variables|/Script/Engine.Character|GetCapsuleComponent _mymech)) false false)))))

(event EventBeginPlay
  (CallFunction|GrabCamera))

(event Input|ActionEvents|InputActionEnter/ExitMech
  (params (Key :type Key%20Structure))
  (:Pressed
    (if (Variables|Default|GetInMech)
      (CallFunction|ExitMech)
      (else
        (CallFunction|EnterMech)))))

(fn ConstructionScript)