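; BP_PersonBullet is a weapon projectile actor that flies in a straight line along its local negative Z axis.
; BeginPlay shrinks the static mesh, then enables its overlap events after a short delay.
; Tick moves the actor by a local offset scaled by world delta seconds, without a projectile movement component.
; It has no active hit handling: the overlap event is a disabled stub, and a SetRelativeLocation node is left unconnected.
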(event EventBeginPlay
  (|CallParentFunction)
  (Transformation|SetWorldScale3D (Variables|Default|GetStaticMesh) "0.050000,0.050000,0.050000")
  (Utilities|FlowControl|Delay 0.2)
  (Variables|/Script/Engine.PrimitiveComponent|SetbGenerateOverlapEvents (Variables|Default|GetStaticMesh) true))

(event Collision|EventActorBeginOverlap
  (params (OtherActor :type Actor%20Object%20Reference))
  (|CallParentFunction OtherActor) ; This node is disabled and will not be called.\nDrag off pins to build functionality.
)

(event EventTick
  (params (DeltaSeconds :type Float%20%28single-precision%29))
  (|CallParentFunction DeltaSeconds)
  (Transformation|AddActorLocalOffset (Math|Vector|MakeVector 0.0 0.0 (* (Utilities|Time|GetWorldDeltaSeconds) -1e+02)) false false))

(fn ConstructionScript
  (|CallParentFunction))