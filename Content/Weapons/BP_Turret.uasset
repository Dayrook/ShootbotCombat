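; BP_Turret is an automatic turret that fires BP_MechBullet projectiles continuously from the start of play.
; BeginPlay calls a Fire event that spawns a bullet at the Arrow component, then calls itself again after FireDelay.
; The sign of the Arrow's world yaw picks the side along world Y for both the spawn offset and the bullet's signed speed.
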(event Custom|Fire
  (bind _arrow (Variables|Default|GetArrow))
  (bind _returnvalue (Transformation|GetWorldRotation _arrow))
  (bind _returnvalue_2 (Transformation|GetWorldLocation _arrow))
  (bind _returnvalue_3 (> (.yaw _returnvalue) 0.0))
  (Utilities|FlowControl|Sequence
    (:then_0
      (bind _returnvalue_4 (Game|SpawnActorfromClass "/Game/Weapons/BP_MechBUllet.BP_MechBullet_C" (Math|Transform|MakeTransform (Math|Vector|MakeVector (.x _returnvalue_2) (+ (.y _returnvalue_2) (select _returnvalue_3 4e+01 -4e+01)) (.z _returnvalue_2)) "0, 0, 0" "1,1,1") "Undefined" 0 0))
      (Variables|/Game/Weapons/BP_BulletBase.BP_BulletBase_C|SetSpeed _returnvalue_4 (select _returnvalue_3 5e+02 -5e+02)))
    (:then_1
      (Utilities|FlowControl|Delay (Variables|Default|GetFireDelay))
      (CallFunction|Fire))))

(event EventBeginPlay
  (CallFunction|Fire))

(fn ConstructionScript)