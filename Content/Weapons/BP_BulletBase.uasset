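; Base bullet actor that flies along its local Y axis at a set speed and damages what it overlaps.
; Spawning plays a sound and briefly delays enabling the overlap box's collision.
; Overlaps skip actors tagged IgnoreBullet or listed in Ignorables, with optional debug prints on valid hits.
; Valid hits receive point damage, then the bullet plays an impact sound and destroys itself after a short delay.
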(event OnComponentBeginOverlap(OverlapBox)
  (params (OverlappedComponent :type Primitive%20Component%20Object%20Reference) (OtherActor :type Actor%20Object%20Reference) (OtherComp :type Primitive%20Component%20Object%20Reference) (OtherBodyIndex :type Integer) (bFromSweep :type Boolean) (SweepResult :type Hit%20Result%20Structure%20%28by%20ref%29))
  ;[1 1 1] Overlap
)

(event Custom|DestroyBullet
  ;[1 1 1] Remove Bullet Actor. TODO: move sound to damaged actor
  (Utilities|IsValid (Variables|Default|GetSoundOnImpact)
    (:Is%20Valid
      (Audio|PlaySound2D (Variables|Default|GetSoundOnImpact) 5.0 1.0 0.0 0 0))
    (:Is%20Not%20Valid
      _))
  (Utilities|FlowControl|Delay 0.1)
  (Actor|DestroyActor))

(event EventBeginPlay
  (Collision|SetCollisionEnabled (Variables|Default|GetOverlapBox) "NoCollision")
  (Audio|PlaySound2D (Variables|Default|GetSoundOnSpawn) 0.6 1.0 0.0 0 0)
  (Utilities|FlowControl|Delay 0.05)
  (Collision|SetCollisionEnabled (Variables|Default|GetOverlapBox) "QueryOnly"))

(event Collision|EventActorBeginOverlap
  (params (OtherActor :type Actor%20Object%20Reference))
  ;[1 1 1] Overlap
  (if (Utilities|IsValid OtherActor)
    (bind _output_get (Variables|Default|SetHitActor OtherActor))
    ;[1 1 1] Valid Target
    (if (not (Utilities|Array|ContainsItem (Variables|/Script/Engine.Actor|GetTags _output_get) "IgnoreBullet"))
      (if (not (Utilities|Array|ContainsItem (Variables|Default|GetIgnorables) (Variables|Default|GetHitActor)))
        (if (Variables|Default|GetDebugMessages)
          ;[1 1 1] Bullet Debugger
          (for _array_element (Variables|Default|GetIgnorables)
            (Development|PrintString (Utilities|String|Append "Ignored : " (Utilities|GetDisplayName _array_element))))
          (Development|PrintString (Utilities|String|Append "Destroyed By : " (Utilities|GetDisplayName (Variables|Default|GetHitActor)))))
        ;[1 1 1] Target Takes Damage
        (Game|Damage|ApplyPointDamage (Variables|Default|GetHitActor) (Variables|Default|GetDamage) (Math|Vector|MakeVector 0.0 (Variables|Default|GetSpeed) 0.0) (Collision|MakeHitResult false false 0.0 0.0 (Transformation|GetWorldLocation (Variables|Default|GetStaticMesh)) "0, 0, 0" "0,0,1" "0,0,1" 0 0) 0 0 "/Script/Engine.DamageType")
        (CallFunction|DestroyBullet)))))

(event EventTick
  (params (DeltaSeconds :type Float%20%28single-precision%29))
  ;[1 1 1] Tick : Movement
  (Transformation|AddActorLocalOffset (Math|Vector|MakeVector 0.0 (* (Variables|Default|GetSpeed) 1.0 (Utilities|Time|GetWorldDeltaSeconds)) 0.0) false false))

(fn ConstructionScript)